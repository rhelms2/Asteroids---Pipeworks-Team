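; BP_Asteroid is a shootable asteroid actor that splits into smaller asteroids when hit by an actor tagged Bullet.
; A hit destroys the bullet, decrements Splits and spawns another BP_Asteroid at SpawnArrow with the same remaining count.
; The new asteroid is scaled down by Scalar, and the original takes that scale reduced once more.
; Tick destroys any asteroid whose Splits count equals zero.
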(event EventBeginPlay
  (Development|PrintString (Utilities|String|ToString(Integer) (Variables|Default|GetSplits)))
  (Variables|Default|SetScalar 0.69))

(event EventTick
  (params (DeltaSeconds :type Float%20%28single-precision%29))
  (Math|Integer|CompareInt (Variables|Default|GetSplits)
    (:==
      (Actor|DestroyActor))))

(event Collision|EventHit
  (params (MyComp :type Primitive%20Component%20Object%20Reference) (Other :type Actor%20Object%20Reference) (OtherComp :type Primitive%20Component%20Object%20Reference) (bSelfMoved :type Boolean) (HitLocation :type Vector :default "0, 0, 0") (HitNormal :type Vector :default "0, 0, 0") (NormalImpulse :type Vector :default "0, 0, 0") (Hit :type Hit%20Result%20Structure%20%28by%20ref%29))
  (if (Actor|ActorHasTag Other "Bullet")
    (Development|PrintString "Asteroid Hit!")
    (Actor|DestroyActor Other)
    (bind _result (Math|Integer|DecrementInt (Variables|Default|GetSplits))
      (:%20%20
        (bind _output_get (Variables|Default|SetSplits _result))
        (Development|PrintString (Utilities|String|ToString(Integer) _output_get))
        (bind _returnvalue (Game|SpawnActorfromClass "BP_Asteroid_C" (Transformation|GetWorldTransform (Variables|Default|GetSpawnArrow)) "Undefined" "OverrideRootScale" 0 (Variables|Default|GetSplits) 0))
        (Transformation|SetActorScale3D _returnvalue (* (Transformation|GetActorScale3D _returnvalue) (Math|Conversions|ToVector(Float) (Variables|Default|GetScalar))))
        (Transformation|SetActorScale3D (* (Transformation|GetActorScale3D _returnvalue) (Math|Conversions|ToVector(Float) (Variables|Default|GetScalar))))))))

(fn ConstructionScript)